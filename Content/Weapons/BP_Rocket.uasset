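; BP_Rocket is a rocket projectile that explodes on impact, or automatically after five seconds in flight.
; On BeginPlay it copies the explosion radius from the first-person player's rocket launcher into its RadialForce component.
; Mesh hits and a Tick-accumulated timer both call Explosion, which fires the radial impulse, spawns an emitter and sound, then destroys the actor.
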(event `self.ReceiveBeginPlay`
  (bind _asbp_first_person_character (cast `/Game/FirstPerson/Blueprints/BP_FirstPersonCharacter` (`GameplayStatics.GetPlayerCharacter` 0)))
  (set `RadialForceComponent.Radius` (`/Game/Weapons/BP_Rocket_Launcher_Component.explosionRadius` (`/Game/FirstPerson/Blueprints/BP_FirstPersonCharacter.RocketLauncherReference` _asbp_first_person_character)) (`self.RadialForce`)))

(event `self.ReceiveTick`
  (params (DeltaSeconds :type "Float (single-precision)"))
  ;[0.05 0.05 0.05] If the rocket projectile doesn't collide with something whithin 5 seconds, then explode automatically
  (bind _output_get (set `self.Timer` (+ (`self.Timer`) DeltaSeconds)))
  (if (>= _output_get 5.0)
    (`self.Explosion` (`self.K2_GetActorLocation`))))

(event `self.StaticMesh.OnComponentHit`
  (params (HitComponent :type "PrimitiveComponent Object Reference") (OtherActor :type "Actor Object Reference") (OtherComp :type "PrimitiveComponent Object Reference") (NormalImpulse :type "Vector Structure") (Hit :type "HitResult Structure (by ref)"))
  ;[0.05 0.05 0.05] Explode Upon Colliding with something
  (`self.Explosion` (`.Location` (`GameplayStatics.BreakHitResult` Hit))))

(fn `Explosion`
  (params (Location :type "Vector Structure"))
  (`RadialForceComponent.FireImpulse` (`self.RadialForce`))
  (`GameplayStatics.SpawnEmitterAtLocation` null Location)
  (`GameplayStatics.PlaySoundAtLocation` null Location (struct) 1.0 1.0 0.0 null null null null)
  (`self.K2_DestroyActor`))

(fn `UserConstructionScript`)