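; Melee weapon component that performs a camera-aimed attack when the shoot input triggers while enabled.
; A visibility line trace out to the attack distance damages "enemy"-tagged actors through the first-person character's HitEnemy and pushes physics-simulating components with an impulse.
; Each swing plays a montage, and a DoOnce reset after the fire-rate delay throttles attacks.
; BeginPlay calls the parent, sets the fire rate and offsets the component's position.
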(event `self.ReceiveBeginPlay`
  (`parent.ReceiveBeginPlay`)
  (`self.SetFirerate` 0.3)
  (`self.K2_SetWorldLocation` (- (`self.K2_GetComponentLocation`) (4.0 7.0 9.0))))

(event `EnhancedInput|/Game/FirstPerson/Input/Actions/IA_Shoot`
  (params (ActionValue :type Boolean) (ElapsedSeconds :type "Float (double-precision)") (TriggeredSeconds :type "Float (double-precision)") (InputAction :type "InputAction Object Reference" :default "/Game/FirstPerson/Input/Actions/IA_Shoot.IA_Shoot"))
  (bind _transformcomponent (`PlayerCameraManager.TransformComponent` (`GameplayStatics.GetPlayerCameraManager` 0)))
  (bind _returnvalue (`self.K2_GetComponentLocation` _transformcomponent))
  (:`Triggered`
    (if (`self.Enabled`)
      (`/Engine/EditorBlueprintResources/StandardMacros.DoOnce` false :!label _label
        (:`Completed`
          (`|ExecutionSequence`
            (:`then_0`
              (bind _outhit (`KismetSystemLibrary.LineTraceSingle` _returnvalue (+ _returnvalue (* (`self.GetForwardVector` _transformcomponent) (`self.AttackDistance`))) "TraceTypeQuery1"))
              (`|ExecutionSequence`
                (:`then_0`
                  (bind (_bblockinghit _binitialoverlap _time _distance _location _impactpoint _normal _impactnormal _physmat _hitactor _hitcomponent) (`GameplayStatics.BreakHitResult` _outhit))
                  ;[1 1 1] Hit tsting for enemy
                  (`/Engine/EditorBlueprintResources/StandardMacros.IsValid` _hitactor
                    (:`Is Valid`
                      (if (`Actor.ActorHasTag` _hitactor "enemy")
                        (bind _asbp_first_person_character (cast `/Game/FirstPerson/Blueprints/BP_FirstPersonCharacter` (`GameplayStatics.GetPlayerCharacter` 0)))
                        (`/Game/FirstPerson/Blueprints/BP_FirstPersonCharacter.hit enemy` _asbp_first_person_character _hitactor (`self.damage dealt`))))
                    (:`Is Not Valid`
                      _))
                  ;[0.05 0.05 0.05] Add impulse to objects with physics
                  (if _bblockinghit
                    (if (`self.IsSimulatingPhysics` _hitcomponent "None")
                      (`self.AddImpulseAtLocation` _hitcomponent (* (`self.GetForwardVector` (`PlayerCameraManager.TransformComponent` (`GameplayStatics.GetPlayerCameraManager` 0))) (`self.Impact`)) _impactpoint "None"))))
                (:`then_1`
                  (`self.PlayMontage` null))))
            (:`then_1`
              (`KismetSystemLibrary.Delay` (`self.GetFirerate`))
              (goto _label :!via `Reset`))))))))