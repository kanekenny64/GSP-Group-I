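; BP_NPC_Exploder is an NPC that makes a one-shot suicide attack on the player.
; Its Attack event waits for AttackSpeed, then applies AttackDamage to the first player's BP_FirstPersonCharacter through ReceiveDamage, prints a debug string and destroys itself.
; The damage has no range check, and a failed character cast leaves the NPC alive.
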(event `self.attack`
  (`KismetSystemLibrary.Delay` (`self.attack speed`))
  (bind _asbp_first_person_character (cast `/Game/FirstPerson/Blueprints/BP_FirstPersonCharacter` (`GameplayStatics.GetPlayerCharacter` 0)))
  (`/Game/FirstPerson/Blueprints/BP_FirstPersonCharacter.Receive Damage` _asbp_first_person_character (`self.attack damage`))
  (`KismetSystemLibrary.PrintString` "explode")
  (`self.K2_DestroyActor`))

(fn `UserConstructionScript`
  (`parent.UserConstructionScript`))