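; BP_NPC_Ranged is a ranged enemy NPC that fires projectiles at the player and destroys itself at zero or lower health.
; Attack sets a flag that makes Tick smoothly rotate the NPC toward the player until nearly aligned.
; It then spawns BP_Enemy_Projectile, passing damage and an upward-biased velocity scaled by player distance, and clears the flag.
; takeDamage overwrites Health with the incoming Damage value instead of subtracting it.
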(event `self.ReceiveBeginPlay`
  (set `CharacterMovementComponent.MaxWalkSpeed` (`self.movementSpeed`) (`self.CharacterMovement`)))

(event `takeDamage`
  (params (damage :type Integer))
  (bind _output_get (set `self.health` damage))
  (if (<= _output_get 0)
    (`self.K2_DestroyActor`)))

(event `self.ReceiveTick`
  (params (DeltaSeconds :type "Float (single-precision)"))
  (bind _returnvalue (`self.K2_GetActorLocation`))
  (bind _returnvalue_2 (`self.K2_GetActorLocation` (`GameplayStatics.GetPlayerCharacter` 0)))
  (bind _returnvalue_3 (`KismetMathLibrary.FindLookAtRotation` _returnvalue _returnvalue_2))
  (bind _returnvalue_4 (`KismetMathLibrary.RInterpTo` (`self.K2_GetActorRotation`) _returnvalue_3 DeltaSeconds 10.0))
  ;[1 1 1] Attacking sequence (rotate then attack)
  (if (`self.attacking`)
    (`self.K2_SetActorRotation` _returnvalue_4)
    (if (== _returnvalue_3 _returnvalue_4 :`ErrorTolerance` 10.0)
      (bind _returnvalue_5 (`|SpawnActorFromClass` "/Game/AI/EnemyProjectiles/BP_Enemy_Projectile.BP_Enemy_Projectile_C" (`KismetMathLibrary.Conv_VectorToTransform` _returnvalue) "Undefined" "MultiplyWithRoot" null null))
      (set `/Game/AI/EnemyProjectiles/BP_Enemy_Projectile.damage` (`self.attack damage`) _returnvalue_5)
      (set `MovementComponent.Velocity` (* (+ (- _returnvalue_2 _returnvalue) (0.0 0.0 50.0)) (100.0 100.0 100.0)) (`ProjectProjectile.ProjectileMovement` _returnvalue_5))
      (set `self.attacking` false))))

(fn `attack`
  (set `self.attacking` true))

(fn `UserConstructionScript`)