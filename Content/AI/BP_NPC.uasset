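; BP_NPC is an AI character Blueprint for a melee NPC that damages the first-person player.
; BeginPlay applies MovementSpeed to the walk speed, while the attack event waits AttackSpeed seconds, then sends AttackDamage to the player without a range check.
; The takeDamage event sets Health to the incoming value rather than subtracting it, destroying the actor at zero or below.
; The RecieveDamage function is an empty stub.
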(event `self.ReceiveBeginPlay`
  (set `CharacterMovementComponent.MaxWalkSpeed` (`self.movementSpeed`) (`self.CharacterMovement`)))

(event `takeDamage`
  (params (damage :type Integer))
  (bind _output_get (set `self.health` damage))
  (if (<= _output_get 0)
    (`self.K2_DestroyActor`)))

(event `attack`
  (`KismetSystemLibrary.Delay` (`self.attack speed`))
  (bind _asbp_first_person_character (cast `/Game/FirstPerson/Blueprints/BP_FirstPersonCharacter` (`GameplayStatics.GetPlayerCharacter` 0)))
  (`/Game/FirstPerson/Blueprints/BP_FirstPersonCharacter.Receive Damage` _asbp_first_person_character (`self.attack damage`))
  (`KismetSystemLibrary.PrintString` "melee attack done"))

(fn `recieve damage`
  (params (damage :type Integer)))

(fn `UserConstructionScript`)